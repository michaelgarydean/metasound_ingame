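; BP_Orb is an orb actor that shifts its audio filtering with the player's proximity.
; Every tick it sets two float parameters on its Audio component, including "Filt Freq Low", using opposite sweep directions.
; A shared helper maps player pawn distance through a clamped, inverted range, shapes it with a power curve, then remaps it to a frequency range.
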(event EventBeginPlay)

(event Collision|EventActorBeginOverlap
  (params (OtherActor :type Actor%20Object%20Reference)))

(event EventTick
  (params (DeltaSeconds :type Float%20%28single-precision%29))
  (bind _audio (Variables|Default|GetAudio))
  (bind _returnvalue (Class|AudioComponent|GetParameterInterface _audio))
  (bind _exponential_distance (CallFunction|FilterFrequencyBasedonDistance 2e+02 2.5e+03 1.15))
  (Class|AudioParameterInterface|SetFloat _returnvalue "Filt Freq Hi" _exponential_distance)
  (bind _exponential_distance_2 (CallFunction|FilterFrequencyBasedonDistance 2e+04 1.5e+03 0.8))
  (Class|AudioParameterInterface|SetFloat _returnvalue "Filt Freq Low" _exponential_distance_2))

(fn ConstructionScript)

(fn FilterFrequencyBasedonDistance
  (params (Min_Freq :type Float%20%28single-precision%29) (Max_Freq :type Float%20%28single-precision%29) (Exp :type Float%20%28single-precision%29))
  (return (Math|Float|MapRangeClamped (Math|Float|Power (Math|Float|MapRangeClamped (Transformation|GetDistanceTo (Game|Player|GetPlayerPawn 0)) 1.2e+03 2e+02 0.0 1.0) Exp) 0.0 1.0 Min_Freq Max_Freq)))