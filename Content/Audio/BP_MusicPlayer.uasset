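; BP_MusicPlayer is an actor that crossfades its audio according to whether something is inside a trigger volume.
; Begin and end overlap on Trigger_Crossfade set an Overlapped flag, sent as a 0/1 float to the Audio component's "Crossfade" parameter.
; A DoOnce gate ignores repeat begin overlaps until any end overlap resets it, without filtering by actor.
; BeginPlay draws a red debug box at the trigger's location.
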(event OnComponentBeginOverlap(Trigger_Crossfade)
  (params (OverlappedComponent :type Primitive%20Component%20Object%20Reference) (OtherActor :type Actor%20Object%20Reference) (OtherComp :type Primitive%20Component%20Object%20Reference) (OtherBodyIndex :type Integer) (bFromSweep :type Boolean) (SweepResult :type Hit%20Result%20Structure%20%28by%20ref%29))
  (Utilities|FlowControl|DoOnce false
    (:Completed
      (Variables|Default|SetOverlapped true)
      (Class|AudioParameterInterface|SetFloat (Class|AudioComponent|GetParameterInterface (Variables|Default|GetAudio)) "Crossfade" (Math|Conversions|ToFloat(Boolean) (Variables|Default|GetOverlapped))))))

(event OnComponentEndOverlap(Trigger_Crossfade)
  (params (OverlappedComponent :type Primitive%20Component%20Object%20Reference) (OtherActor :type Actor%20Object%20Reference) (OtherComp :type Primitive%20Component%20Object%20Reference) (OtherBodyIndex :type Integer))
  (Utilities|FlowControl|Sequence
    (:then_0
      (Utilities|FlowControl|DoOnce false) ; enters at Reset
    )
    (:then_1
      (Variables|Default|SetOverlapped false)
      (Class|AudioParameterInterface|SetFloat (Class|AudioComponent|GetParameterInterface (Variables|Default|GetAudio)) "Crossfade" (Math|Conversions|ToFloat(Boolean) (Variables|Default|GetOverlapped))))))

(event EventBeginPlay
  (Rendering|Debug|DrawDebugBox (Transformation|GetWorldLocation (Variables|Default|GetTrigger_Crossfade)) "0, 0, 0" "(R=1.000000,G=0.000000,B=0.000000,A=1.000000)" "0, 0, 0" 0.0 4.0))

(event Collision|EventActorBeginOverlap
  (params (OtherActor :type Actor%20Object%20Reference)))

(event EventTick
  (params (DeltaSeconds :type Float%20%28single-precision%29)))

(fn ConstructionScript)